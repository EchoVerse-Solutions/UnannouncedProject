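; BP_MyGameMode is a game mode that handles main menu startup and the transition into the first prototype level.
; On BeginPlay it shows the mouse cursor in every level, then creates, stores and displays UI_MainMenu only when the level is MainMenu.
; OnPrototypeLevel1Load opens PrototypeLevel1 and sets game-only input; an author note says this logic currently lives in the NewGame button and still needs binding here.
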(event `self.ReceiveBeginPlay`
  (set `PlayerController.bShowMouseCursor` true (`GameplayStatics.GetPlayerController` 0))
  (bind _returnvalue (`GameplayStatics.GetCurrentLevelName` true))
  (if (`KismetStringLibrary.EqualEqual_StrStr` _returnvalue "MainMenu")
    (bind _returnvalue_2 (`|CreateWidget` "/Game/Content/UI/MainMenu/UI_MainMenu.UI_MainMenu_C"))
    (bind _output_get (set `self.Main Menu Ref` _returnvalue_2))
    (`UserWidget.AddToViewport` _output_get 0)))

(event `On Prototype Level 1 Load`
  ;[1 0.0279 0] Сейчас вся логика в кнопке NewGame Button. надо будет привязать сюда
  (`GameplayStatics.OpenLevel` "PrototypeLevel1")
  (`WidgetBlueprintLibrary.SetInputMode_GameOnly` (`GameplayStatics.GetPlayerController` 0)))

(fn `UserConstructionScript`)